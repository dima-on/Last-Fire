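; BP_Wearpon is a weapon pickup that spins on its yaw each tick and respawns after being collected.
; On overlap it hides and disables collision, then passes its index, material and mesh to BP_Player through PickUpServer.
; A timer restores visibility and collision 15 seconds later.
; Hiding precedes the player cast, so a non-player overlap hides it without starting that timer.
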(event `self.ReceiveTick`
  (params (DeltaSeconds :type "Float (single-precision)"))
  (bind _wearpon (`self.Wearpon`))
  (bind (_returnvalue_roll _returnvalue_pitch _returnvalue_yaw) (`KismetMathLibrary.BreakRotator` (`SceneComponent.K2_GetComponentRotation` _wearpon)))
  (`SceneComponent.K2_SetWorldRotation` _wearpon (`KismetMathLibrary.MakeRotator` _returnvalue_roll _returnvalue_pitch (+ _returnvalue_yaw 1.0)) false false))

(event `self.Wearpon.OnComponentBeginOverlap`
  (params (OverlappedComponent :type "PrimitiveComponent Object Reference") (OtherActor :type "Actor Object Reference") (OtherComp :type "PrimitiveComponent Object Reference") (OtherBodyIndex :type Integer) (bFromSweep :type Boolean) (SweepResult :type "HitResult Structure (by ref)"))
  (bind _wearpon (`self.Wearpon`))
  (`SceneComponent.SetHiddenInGame` (`self.Wearpon`) true false)
  (`PrimitiveComponent.SetCollisionEnabled` (`self.Wearpon`) "NoCollision")
  (bind _asbp_player (cast `/Game/Blueprints/Player_Blueprints/BP_Player` OtherActor))
  (`/Game/Blueprints/Player_Blueprints/BP_Player.Pick Up Server` _asbp_player (`self.Index`) (`PrimitiveComponent.GetMaterial` _wearpon 0) (`StaticMeshComponent.StaticMesh` _wearpon))
  (`KismetSystemLibrary.K2_SetTimerDelegate` (delegate `Create Wearpone`) 15.0))

(event `Create Wearpone`
  (`SceneComponent.SetHiddenInGame` (`self.Wearpon`) false false)
  (`PrimitiveComponent.SetCollisionEnabled` (`self.Wearpon`) "QueryAndPhysics"))

(fn `UserConstructionScript`)