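; AC_Wearpon is a weapon component, judging by its name, that calculates damage based on distance.
; On BeginPlay it precomputes a per-meter slope between Damage and DistanceDamage over 100 meters.
; CalDistanceDamage converts a distance in centimeters to meters and interpolates linearly with that slope, returning DistanceDamage from 100 meters onward.
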(event `self.ReceiveBeginPlay`
  (set `self.Kof_Distance` (/ (- (`self.Distance_Damage`) (`self.Damage`)) 100.0)))

(fn `Cal Distance Damage`
  (params (Distance :type "Float (double-precision)"))
  (returns (output_damage :type "Float (double-precision)"))
  (if (< Distance 10000.0)
    (return (+ (* (/ Distance 100.0) (`self.Kof_Distance`)) (`self.Damage`)))
    (else
      (return (`self.Distance_Damage`)))))